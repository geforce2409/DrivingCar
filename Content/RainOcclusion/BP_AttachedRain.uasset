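; BP_AttachedRain is a rain actor that follows the player pawn, teleporting to its location every tick.
; Shortly after BeginPlay it reads IsRainy from MyPlayerController to show or hide itself, play or stop its audio, and toggle the controller's Chameleon reference.
; On construction and every tick it writes its up vector and rain particle location into the MPC_RainDepth material parameter collection.
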(event Custom|PopulateCollectionParameters
  (Rendering|Material|SetVectorParameterValue "/Game/RainOcclusion/MPC_RainDepth.MPC_RainDepth" "UpVector" (Math|Conversions|ToLinearColor(Vector) (Transformation|GetActorUpVector)) :!class /Script/Engine.KismetMaterialLibrary)
  (Rendering|Material|SetVectorParameterValue "/Game/RainOcclusion/MPC_RainDepth.MPC_RainDepth" "ParticleLocation" (Math|Conversions|ToLinearColor(Vector) (Transformation|GetWorldLocation (Variables|Default|GetPS_Rain))) :!class /Script/Engine.KismetMaterialLibrary))

(event EventBeginPlay
  (bind _audio (Variables|Default|GetAudio))
  (bind _asmy_player_controller (Utilities|Casting|CastToMyPlayerController (Game|GetPlayerController 0)))
  (Utilities|FlowControl|Delay 0.2)
  (if (Variables|/Game/Blueprints/MyPlayerController.MyPlayerController_C|GetisRainy? _asmy_player_controller)
    (Rendering|SetActorHiddenInGame false)
    (Audio|Components|Audio|Play _audio 0.0)
    (Variables|/Game/Chameleon/Chameleon.Chameleon_C|SetEnabled (Variables|/Game/Blueprints/MyPlayerController.MyPlayerController_C|GetChameleonReference _asmy_player_controller) true)
    (else
      (Rendering|SetActorHiddenInGame true)
      (Audio|Components|Audio|Stop _audio)
      (Variables|/Game/Chameleon/Chameleon.Chameleon_C|SetEnabled (Variables|/Game/Blueprints/MyPlayerController.MyPlayerController_C|GetChameleonReference _asmy_player_controller) false))))

(event Collision|EventActorBeginOverlap
  (params (OtherActor :type Actor%20Object%20Reference)))

(event EventTick
  (params (DeltaSeconds :type Float%20%28single-precision%29))
  (CallFunction|PopulateCollectionParameters)
  (Transformation|SetActorLocation (Transformation|GetActorLocation (Game|Player|GetPlayerPawn 0)) false false))

(fn ConstructionScript
  (CallFunction|PopulateCollectionParameters))