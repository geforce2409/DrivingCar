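; Game mode for Time Attack that spawns the player's selected car and holds it until the race starts.
; On BeginPlay it spawns the car class stored in BP_GameInstance at a player start, possesses it, then handbrakes and disables input on every BP_Master_Vehicle.
; Tick polls MyPlayerController's RaceStart flag, then releases only the player's vehicle and switches its own tick off.
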(event EventBeginPlay
  (bind _asbp_game_instance (Utilities|Casting|CastToBP_GameInstance (Game|GetGameInstance)))
  (bind _returnvalue (Game|SpawnActorfromClass (Variables|/Game/CustomPhysicVehicle/BP_GameInstance.BP_GameInstance_C|GetSelected%20Car _asbp_game_instance) (Transformation|GetActorTransform (Class|GameModeBase|FindPlayerStart)) "AdjustIfPossibleButAlwaysSpawn" 0 false true true true true true true false false false false false false 1.0 1.5 0.0 "/Game/CustomPhysicVehicle/Vehicles/00_Master_Vehicle/Materials/M_default.M_default" 0 true 0))
  (Variables|/Game/CustomPhysicVehicle/Vehicles/00_Master_Vehicle/BP_Master_Vehicle.BP_Master_Vehicle_C|SetAuto%20Rotate%20Camera _returnvalue false)
  (Pawn|Possess (Game|GetPlayerController 0) _returnvalue)
  (bind _outactors (Actor|GetAllActorsOfClass "/Game/CustomPhysicVehicle/Vehicles/00_Master_Vehicle/BP_Master_Vehicle.BP_Master_Vehicle_C"))
  (for _array_element _outactors
    (Default|ServerHandbrake _array_element true)
    (Input|DisableInput _array_element 0)))

(event EventTick
  (params (DeltaSeconds :type Float%20%28single-precision%29))
  (bind _returnvalue (Game|Player|GetPlayerPawn 0))
  (bind _asbp_master_vehicle (Utilities|Casting|CastToBP_Master_Vehicle _returnvalue))
  ;[1 1 1] Check player start the game or not then enable input and disable event tick
  (if (Variables|/Game/Blueprints/MyPlayerController.MyPlayerController_C|GetRaceStart (.AsMy%20Player%20Controller (Utilities|Casting|CastToMyPlayerController (Game|GetPlayerController 0))))
    (Default|ServerHandbrake _asbp_master_vehicle false)
    (Input|EnableInput _asbp_master_vehicle 0)
    (Actor|Tick|SetActorTickEnabled false)))

(fn ConstructionScript)