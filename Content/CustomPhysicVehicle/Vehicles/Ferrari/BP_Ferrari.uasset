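; Player-drivable Ferrari vehicle Blueprint that builds on a parent vehicle class.
; Routes driving, exit, headlight and turbo input to parent Server functions, while view switching and look-around input stay local.
; Feeds steering angle to car and driver animation Blueprints on Tick, or hides the scene mirror instead when an AI controller class is set.
; Renders the mirror through a scene capture, runtime render target and dynamic material.
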(event EventBeginPlay
  (|CallParentFunction)
  (|HandlingAnimationBlueprints)
  (|Mirrors))

(event EventTick
  (params (DeltaSeconds :type Float%20%28single-precision%29))
  (CallFunction|LookAround (Input|AxisValues|GetLookUp) (Input|AxisValues|GetLookRight))
  (CallFunction|ServerTick)
  (if (Utilities|IsValidClass (Variables|Default|GetAIControllerClass))
    (Utilities|FlowControl|DoOnce false
      (:Completed
        (Rendering|SetVisibility (Variables|Default|GetSceneMIrror) false false)))
    (else
      (|UpdateAnimationBlueprints))))

(event Input|ActionEvents|InputActionHandbrake
  (params (Key :type Key%20Structure :default "None"))
  ;[0 0.51 0.02325] Network Relevant Inputs
  (:Pressed
    (CallFunction|ServerHandbrake true))
  (:Released
    (CallFunction|ServerHandbrake false)))

(event Input|ActionEvents|InputActionSwitchHeadLight
  (params (Key :type Key%20Structure :default "None"))
  ;[0 0.51 0.02325] Network Relevant Inputs
  (:Pressed
    (CallFunction|ServerHeadLights)))

(event Input|ActionEvents|InputActionInteract
  (params (Key :type Key%20Structure :default "None"))
  ;[0 0.51 0.02325] Network Relevant Inputs
  (:Pressed
    (CallFunction|ServerExitVehicle)))

(event Input|ActionEvents|InputActionSwitchCamera
  (params (Key :type Key%20Structure :default "None"))
  ;[0 0.2691 1] Local Only Inputs
  (:Pressed
    (CallFunction|ChangeView)))

(event Input|ActionEvents|InputActionVehicle_ViewRear
  (params (Key :type Key%20Structure :default "None"))
  ;[0 0.2691 1] Local Only Inputs
  (:Pressed
    (Variables|Default|SetLook%20Back true))
  (:Released
    (Variables|Default|SetLook%20Back false)
    (Variables|Default|SetFP%20Camera%20Returning? true)))

(event Input|ActionEvents|InputActionVehicle_ViewLeft
  (params (Key :type Key%20Structure :default "None"))
  ;[0 0.2691 1] Local Only Inputs
  (:Pressed
    (Variables|Default|SetLook%20Left true))
  (:Released
    (Variables|Default|SetLook%20Left false)
    (Variables|Default|SetFP%20Camera%20Returning? true)))

(event Input|ActionEvents|InputActionVehicle_ViewRight
  (params (Key :type Key%20Structure :default "None"))
  ;[0 0.2691 1] Local Only Inputs
  (:Pressed
    (Variables|Default|SetLook%20Right true))
  (:Released
    (Variables|Default|SetLook%20Right false)
    (Variables|Default|SetFP%20Camera%20Returning? true)))

(event Input|ActionEvents|InputActionGearUp
  (params (Key :type Key%20Structure :default "None"))
  ;[0 0.2691 1] Local Only Inputs
)

(event Input|ActionEvents|InputActionGearDown
  (params (Key :type Key%20Structure :default "None"))
  ;[0 0.2691 1] Local Only Inputs
)

(event Input|ActionEvents|InputActionTurboBoost
  (params (Key :type Key%20Structure :default "None"))
  ;[0 0.51 0.02325] Network Relevant Inputs
  (:Pressed
    (if (Variables|Default|GetIs%20Accelerating)
      (Audio|Components|Audio|Play (Variables|Default|GetNitroSound) 0.0))))

(event Input|AxisEvents|InputAxisMoveBack
  (params (AxisValue :type Float%20%28single-precision%29))
  ;[0 0.51 0.02325] Network Relevant Inputs
  (CallFunction|ServerBrake AxisValue false))

(event Input|AxisEvents|InputAxisMoveRight
  (params (AxisValue :type Float%20%28single-precision%29))
  ;[0 0.51 0.02325] Network Relevant Inputs
  (CallFunction|ServerSteering AxisValue (* (Input|AxisValues|GetLookRight) 2.0)))

(event Input|AxisEvents|InputAxisMoveForward
  (params (AxisValue :type Float%20%28single-precision%29))
  ;[0 0.51 0.02325] Network Relevant Inputs
  (CallFunction|ServerThrottle AxisValue))

(event Input|AxisEvents|InputAxisTurboBoost
  (params (AxisValue :type Float%20%28single-precision%29))
  ;[0 0.51 0.02325] Network Relevant Inputs
  (CallFunction|ServerTurboBoost AxisValue))

(event Input|KeyboardEvents|Q
  (params (Key :type Key%20Structure :default "None"))
  ;[0 0.51 0.02325] Network Relevant Inputs
  (:Pressed
    (CallFunction|ServerReverseGear true))
  (:Released
    (CallFunction|ServerReverseGear false)))

(event Input|KeyboardEvents|Tab
  (params (Key :type Key%20Structure :default "None"))
  ;[0 0.2691 1] Local Only Inputs
  (:Pressed
    (if (Variables|Default|GetCan%20Display%20Debug%20Widget)
      (Utilities|FlowControl|FlipFlop
        (:A
          (CallFunction|DebugWidget true))
        (:B
          (CallFunction|DebugWidget false))))))

(fn ConstructionScript
  (|CallParentFunction))