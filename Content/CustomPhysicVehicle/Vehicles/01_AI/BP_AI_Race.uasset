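; AI controller that races a BP_Master_Vehicle along the "Race"-tagged track spline once the race starts, under a random driver name.
; A half-second timer detects opponents ahead, steering angle and drifting, then derives desired speed, throttle and brake.
; Steering targets a speed-scaled look-ahead spline point, shifted sideways around the closest opponent.
; Speed drops for upcoming curves and blocking cars; Tick sends the inputs to the vehicle.
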(event Custom|Timer_01
  (CallFunction|DetectOpponents)
  (CallFunction|HandleSteeringAngle)
  (CallFunction|DetectDrifting)
  (CallFunction|CalculateDesiredSpeed)
  (CallFunction|HandleSpeed))

(event EventBeginPlay
  (Variables|Default|SetName (Utilities|Select :Index (Math|Random|RandomIntegerinRange 0 12) :Option%200 "Paul" :Option%201 "Gavin" :Option%202 "Kelly" :Option%203 "Kevin" :Option%204 "Mathieu" :Option%205 "Alex" :Option%206 "Bob" :Option%207 "Robert" :Option%208 "Steeve" :Option%209 "Cosimo" :Option%2010 "Samuel" :Option%2011 "Oti" :Option%2012 "Andrew"))
  (bind _asbp_master_vehicle (Utilities|Casting|CastToBP_Master_Vehicle (Pawn|GetControlledPawn self)))
  (bind _output_get (Variables|Default|SetVehicle _asbp_master_vehicle))
  (Variables|Default|SetCarName (Utilities|Text|ToText(Name) (Utilities|Array|Get(acopy) (Variables|/Script/Engine.Actor|GetTags _output_get) 1))))

(event EventTick
  (params (DeltaSeconds :type Float%20%28single-precision%29))
  (bind _vehicle (Variables|Default|GetVehicle))
  (Utilities|FlowControl|Sequence
    (:then_0
      (if (Variables|/Game/Blueprints/MyPlayerController.MyPlayerController_C|GetRaceStart (.AsMy%20Player%20Controller (Utilities|Casting|CastToMyPlayerController (Game|GetPlayerController 0))))
        (Utilities|FlowControl|DoOnce false
          (:Completed
            (CallFunction|Begin)
            (Utilities|Time|SetTimerbyFunctionName 0 "Timer_01" 0.5 true)
            (bind _returnvalue (AddComponent|AddTextRenderComponent (Variables|Default|GetVehicle) false (Math|Transform|MakeTransform "0, 0,185.000000" "0,180.000000, 0" "1,1,1")))
            (Rendering|Components|TextRender|SetText _returnvalue (Variables|Default|GetName))))))
    (:then_1
      (Utilities|IsValid _vehicle
        (:Is%20Valid
          (Default|ServerThrottle _vehicle (Variables|Default|GetThrottle%20Input))
          (Default|ServerBrake _vehicle (Variables|Default|GetBrake%20Input) false)
          (Default|ServerSteering _vehicle (Variables|Default|GetSteering%20Input) 0.0))))))

(fn ConstructionScript)

(fn Begin
  (bind _vehicle (Variables|Default|GetVehicle))
  (Default|PossessVehicle (Variables|Default|GetVehicle) self)
  (Rendering|SetVisibility (Variables|/Game/CustomPhysicVehicle/Vehicles/00_Master_Vehicle/BP_Master_Vehicle.BP_Master_Vehicle_C|GetDriver (Variables|Default|GetVehicle)) true true)
  (bind _outactors (Actor|GetAllActorswithTag "Race"))
  (bind _asbp_track_spline (Utilities|Casting|CastToBP_Track_Spline (Utilities|Array|Get(acopy) _outactors)))
  (Variables|Default|SetTrack%20to%20Follow _asbp_track_spline)
  (Transformation|AttachComponentToComponent (Variables|Default|GetOpponent%20Sphere%20Detection) (Variables|/Game/CustomPhysicVehicle/Vehicles/00_Master_Vehicle/BP_Master_Vehicle.BP_Master_Vehicle_C|GetMesh (Variables|Default|GetVehicle)) "None" "SnapToTarget" "SnapToTarget" "KeepRelative" true)
  (bind _array_element (Utilities|Array|ForEachLoopwithBreak (Variables|/Game/CustomPhysicVehicle/Vehicles/00_Master_Vehicle/BP_Master_Vehicle.BP_Master_Vehicle_C|GetWheels (Variables|Default|GetVehicle)) :!label _label)
    (:LoopBody
      (if (not (== (.SteeringAngle (Utilities|Struct|BreakWheel_Structure _array_element)) 0.0))
        (Utilities|FlowControl|Sequence
          (:then_0
            (goto _label Break))
          (:then_1
            (Variables|Default|SetMaximum%20Steering (Math|Float|Absolute(Float) (.SteeringAngle (Utilities|Struct|BreakWheel_Structure _array_element))))))))
    (:Completed
      (Variables|/Game/CustomPhysicVehicle/Vehicles/00_Master_Vehicle/BP_Master_Vehicle.BP_Master_Vehicle_C|SetAutomatic%20Transmision _vehicle true)
      (Variables|/Game/CustomPhysicVehicle/Vehicles/00_Master_Vehicle/BP_Master_Vehicle.BP_Master_Vehicle_C|SetBrake%20as%20Reverse _vehicle true)
      (Variables|/Game/CustomPhysicVehicle/Vehicles/00_Master_Vehicle/BP_Master_Vehicle.BP_Master_Vehicle_C|SetGear _vehicle 2))))

(fn PrintDebugVariables
  (bind _vehicle (Variables|Default|GetVehicle))
  (Utilities|IsValid (Variables|Default|GetVehicle)
    (:Is%20Valid
      (Rendering|Debug|DrawDebugSphere (Variables|Default|GetTarget%20Location) 1e+02 12 "(R=1.000000,G=1.000000,B=1.000000,A=1.000000)" 0.0)
      (Rendering|Debug|DrawDebugString (+ (Transformation|GetActorLocation (Variables|Default|GetVehicle)) "0, 0,200.000000") (Utilities|String|SelectString "Accelerating!" "" (Variables|Default|GetIs%20Accelerating)) 0 "(R=0.085258,G=0.541667,B=0.000000,A=1.000000)")
      (Rendering|Debug|DrawDebugString (+ (Transformation|GetActorLocation (Variables|Default|GetVehicle)) "0, 0,180.000000") (Utilities|String|SelectString "Braking!" "" (Variables|Default|GetIs%20Braking)) 0 "(R=0.085258,G=0.541667,B=0.000000,A=1.000000)")
      (Rendering|Debug|DrawDebugString (+ (Transformation|GetActorLocation (Variables|Default|GetVehicle)) "0, 0,120.000000") (Utilities|String|SelectString (Utilities|String|Append (Utilities|String|ToString(Integer) (Math|Float|Round (Variables|Default|GetDrift%20Angle))) "°" "  Drift") "" (Variables|Default|GetIs%20Drifting)) 0 "(R=0.085258,G=0.541667,B=0.000000,A=1.000000)")
      (Rendering|Debug|DrawDebugString (+ (Transformation|GetActorLocation (Variables|Default|GetVehicle)) "0, 0,100.000000") (Utilities|String|Append "Steering Angle : " (Utilities|String|ToString(Integer) (Math|Float|Round (Variables|Default|GetSteering%20Angle)))) 0 "(R=0.085258,G=0.541667,B=0.000000,A=1.000000)")
      (Rendering|Debug|DrawDebugString (+ (Transformation|GetActorLocation (Variables|Default|GetVehicle)) "0, 0,80.000000") (Utilities|String|Append "Speed (km/h) : " (Utilities|String|ToString(Integer) (Math|Float|Round (* (Math|Vector|VectorLength (Transformation|GetVelocity (Variables|Default|GetVehicle))) 0.036)))) 0 "(R=0.085258,G=0.541667,B=0.000000,A=1.000000)")
      (Rendering|Debug|DrawDebugString (+ (Transformation|GetActorLocation (Variables|Default|GetVehicle)) "0, 0,60.000000") (Utilities|String|Append "Gear : " (.gearname (Utilities|Array|Get(acopy) (Variables|/Game/CustomPhysicVehicle/Vehicles/00_Master_Vehicle/BP_Master_Vehicle.BP_Master_Vehicle_C|GetGears _vehicle) (Variables|/Game/CustomPhysicVehicle/Vehicles/00_Master_Vehicle/BP_Master_Vehicle.BP_Master_Vehicle_C|GetGear _vehicle)))) 0 "(R=0.085258,G=0.541667,B=0.000000,A=1.000000)")
      ;[1 1 1] Print Opponents Debug Info
      (for _array_element (Variables|Default|GetSeen%20Opponents)
        (if (Utilities|IsValid (.OpponentActor (Utilities|Struct|BreakAI_Opponents_Struct _array_element)))
          (Rendering|Debug|DrawDebugSphere (Transformation|GetActorLocation (.OpponentActor (Utilities|Struct|BreakAI_Opponents_Struct _array_element))) 2.5e+02 12 "(R=1.000000,G=1.000000,B=1.000000,A=1.000000)" 0.0)
          (Rendering|Debug|DrawDebugString (Transformation|GetActorLocation (.OpponentActor (Utilities|Struct|BreakAI_Opponents_Struct _array_element))) (Utilities|String|Append (Utilities|String|ToString(Integer) (Math|Float|Round (.OpponentDistance (Utilities|Struct|BreakAI_Opponents_Struct _array_element)))) " cm.") 0 "(R=1.000000,G=1.000000,B=1.000000,A=1.000000)")
          (Rendering|Debug|DrawDebugString (+ (Transformation|GetActorLocation (.OpponentActor (Utilities|Struct|BreakAI_Opponents_Struct _array_element))) "0, 0,20.000000") (Utilities|String|Append (Utilities|String|ToString(Integer) (Math|Float|Round (.OpponentAngle (Utilities|Struct|BreakAI_Opponents_Struct _array_element)))) " deg.") 0 "(R=1.000000,G=1.000000,B=1.000000,A=1.000000)"))))))

(fn HandleSteeringAngle
  (bind (_steering_angle _target_location _curve_anticipation) (|CalculateSteeringAngle(NoOpponent)))
  (bind (_steering_angle_2 _target_location_2 _curve_anticipation_2) (|CalculateSteeringAngle))
  (Utilities|IsValid (Variables|Default|GetVehicle)
    (:Is%20Valid
      (if (Utilities|Array|IsValidIndex (Variables|Default|GetSeen%20Opponents))
        (Variables|Default|SetSteering%20Angle _steering_angle_2)
        (Variables|Default|SetTarget%20Location _target_location_2)
        (Variables|Default|SetCurve%20Anticipate _curve_anticipation_2)
        (else
          (Variables|Default|SetSteering%20Angle _steering_angle)
          (Variables|Default|SetTarget%20Location _target_location)
          (Variables|Default|SetCurve%20Anticipate _curve_anticipation)))
      (Variables|Default|SetSteering%20Input (|ConvertsteeringangleintoSteeringInput)))))

(fn HandleSpeed
  (bind _should_accelerate (Variables|Default|GetShould%20accelerate))
  (bind _vehicle (Variables|Default|GetVehicle))
  (bind _desired_speed (Variables|Default|GetDesired%20Speed))
  (bind _desired_speed_2 (Variables|Default|GetDesired%20Speed))
  (bind _steering_angle (Variables|Default|GetSteering%20Angle))
  (bind _maximum_steering (Variables|Default|GetMaximum%20Steering))
  (bind _returnvalue (Math|Float|Absolute(Float) _steering_angle))
  (bind _returnvalue_2 (Transformation|GetVelocity _vehicle))
  (bind _returnvalue_3 (- _desired_speed_2 1e+01))
  (bind _returnvalue_4 (+ _maximum_steering 2e+01))
  (bind _returnvalue_5 (+ _desired_speed 5e+01))
  (bind _returnvalue_6 (+ _desired_speed 15.0))
  (bind _returnvalue_7 (> _returnvalue _returnvalue_4))
  (bind _returnvalue_8 (Math|Vector|VectorLength _returnvalue_2))
  (bind _returnvalue_9 (Math|Float|SelectFloat 0.0 1.0 _returnvalue_7))
  (bind _returnvalue_10 (* _returnvalue_8 0.036))
  (bind _returnvalue_11 (Math|Float|MapRangeClamped _returnvalue_10 _returnvalue_6 _returnvalue_5 0.0 0.5))
  (bind _returnvalue_12 (Math|Float|SelectFloat _returnvalue_9 0.0 _should_accelerate))
  (bind _returnvalue_13 (Math|Float|MapRangeClamped _returnvalue_10 _returnvalue_3 _desired_speed_2 _returnvalue_12 0.0))
  (Utilities|IsValid (Variables|Default|GetVehicle)
    (:Is%20Valid
      (if (Variables|Default|GetIs%20Drifting)
        (Variables|Default|SetThrottle%20Input 0.0)
        (Variables|Default|SetBrake%20Input 0.0)
        (if (> (Variables|/Game/CustomPhysicVehicle/Vehicles/00_Master_Vehicle/BP_Master_Vehicle.BP_Master_Vehicle_C|GetGear (Variables|Default|GetVehicle)) 2)
          (Default|GearDown (Variables|Default|GetVehicle)))
        (elif (> _returnvalue_10 (+ (Variables|Default|GetDesired%20Speed) 1.0))
          (Variables|Default|SetThrottle%20Input 0.0)
          (Variables|Default|SetIs%20Accelerating false)
          (if (and (> _returnvalue_10 (+ (Variables|Default|GetDesired%20Speed) 1e+01)) (not (Variables|Default|GetIs%20Drifting)))
            (Variables|Default|SetBrake%20Input _returnvalue_11)
            (Variables|Default|SetIs%20Braking (> _returnvalue_11 0.1)))
          (else
            (Variables|Default|SetThrottle%20Input _returnvalue_13)
            (Variables|Default|SetIs%20Accelerating (> _returnvalue_13 0.1))
            (Variables|Default|SetIs%20Braking false)
            (Variables|Default|SetBrake%20Input (Math|Float|SelectFloat 1.0 0.0 (> (Math|Float|Absolute(Float) (Variables|Default|GetSteering%20Angle)) (+ (Variables|Default|GetMaximum%20Steering) 2e+01))))))))))

(fn DetectDrifting
  (bind _vehicle (Variables|Default|GetVehicle))
  (bind _vehicle_2 (Variables|Default|GetVehicle))
  (bind _mesh (Variables|/Game/CustomPhysicVehicle/Vehicles/00_Master_Vehicle/BP_Master_Vehicle.BP_Master_Vehicle_C|GetMesh _vehicle_2))
  (Utilities|IsValid (Variables|Default|GetVehicle)
    (:Is%20Valid
      (bind _output_get (Variables|Default|SetDrift%20Angle (Math|Float|Absolute(Float) (.yaw (Math|Conversions|RotationFromXVector (Math|Transform|InverseTransformDirection (Transformation|GetWorldTransform _mesh) (Transformation|GetComponentVelocity _mesh)))))))
      (Variables|Default|SetIs%20Drifting (and (>= _output_get 3.0) (< (+ (* (Math|Vector|VectorLength (Transformation|GetVelocity _vehicle)) 0.036) 1e+01) (Math|Float|Absolute(Float) (Variables|/Game/CustomPhysicVehicle/Vehicles/00_Master_Vehicle/BP_Master_Vehicle.BP_Master_Vehicle_C|GetSpeed _vehicle))))))))

(fn CalculateDesiredSpeed
  (bind _seen_opponents (Variables|Default|GetSeen%20Opponents))
  (bind _vehicle (Variables|Default|GetVehicle))
  (bind _curve_anticipate (Variables|Default|GetCurve%20Anticipate))
  (bind _most_in_front_opponent_index (Variables|Default|GetMost%20in%20Front%20Opponent%20Index))
  (bind _returnvalue (Math|Float|Absolute(Float) _curve_anticipate))
  (bind _output (Utilities|Array|Get(acopy) _seen_opponents _most_in_front_opponent_index))
  (bind _ai_min_speed (Variables|/Game/CustomPhysicVehicle/Vehicles/00_Master_Vehicle/BP_Master_Vehicle.BP_Master_Vehicle_C|GetAI%20Min%20Speed _vehicle))
  (bind _ai_max_speed (Variables|/Game/CustomPhysicVehicle/Vehicles/00_Master_Vehicle/BP_Master_Vehicle.BP_Master_Vehicle_C|GetAI%20Max%20Speed _vehicle))
  (bind (_opponentactor _opponentdistance _opponentangle) (Utilities|Struct|BreakAI_Opponents_Struct _output))
  (bind _returnvalue_2 (Math|Float|MapRangeClamped _returnvalue 4.0 15.0 _ai_max_speed _ai_min_speed))
  (Utilities|IsValid (Variables|Default|GetVehicle)
    (:Is%20Valid
      (if (Utilities|Array|IsValidIndex _seen_opponents)
        (Variables|Default|SetDesired%20Speed (Math|Float|Clamp(Float) _returnvalue_2 _ai_min_speed (Math|Float|Lerp _ai_max_speed (Math|Float|Lerp (* (Math|Vector|VectorLength (Transformation|GetVelocity _opponentactor)) 0.0036) _ai_max_speed (Math|Float|MapRangeClamped _opponentdistance 6e+02 1e+03 0.0 1.0)) (Math|Float|MapRangeClamped (Math|Float|Absolute(Float) _opponentangle) 5.0 15.0 1.0 0.0))))
        (else
          (Variables|Default|SetDesired%20Speed _returnvalue_2))))))

(fn HandleGears
  (Utilities|IsValid (Variables|Default|GetVehicle)
    (:Is%20Valid
      (if (> (Variables|Default|GetDesired%20Speed) 5e+01)
        (Variables|/Game/CustomPhysicVehicle/Vehicles/00_Master_Vehicle/BP_Master_Vehicle.BP_Master_Vehicle_C|SetGear (Variables|Default|GetVehicle) 3)
        (elif (<= (Variables|Default|GetDesired%20Speed) 5e+01)
          (Variables|/Game/CustomPhysicVehicle/Vehicles/00_Master_Vehicle/BP_Master_Vehicle.BP_Master_Vehicle_C|SetGear (Variables|Default|GetVehicle) 2))))))

(fn DetectOpponents
  (bind _vehicle (Variables|Default|GetVehicle))
  (bind _returnvalue (Transformation|GetActorForwardVector _vehicle))
  (Utilities|IsValid (Variables|Default|GetVehicle)
    (:Is%20Valid
      (Utilities|Array|Clear (Variables|Default|GetSeen%20Opponents))
      (for _array_element (Collision|GetOverlappingActors (Variables|Default|GetOpponent%20Sphere%20Detection) "/Game/CustomPhysicVehicle/Vehicles/00_Master_Vehicle/BP_Master_Vehicle.BP_Master_Vehicle_C" :!class /Script/Engine.PrimitiveComponent)
        (if (< (Class|KismetMathLibrary|DegAcos (Math|Vector|DotProduct (Math|Vector|Normalize (- (Transformation|GetActorLocation _array_element) (Transformation|GetActorLocation _vehicle))) _returnvalue)) 9e+01)
          (Utilities|Array|Add (Variables|Default|GetSeen%20Opponents) (Utilities|Struct|MakeAI_Opponents_Struct _array_element (Math|Vector|VectorLength (- (Transformation|GetActorLocation _array_element) (Transformation|GetActorLocation _vehicle))) (* (Class|KismetMathLibrary|DegAcos (Math|Vector|DotProduct (Math|Vector|Normalize (- (Transformation|GetActorLocation _array_element) (Transformation|GetActorLocation _vehicle))) _returnvalue)) (.z (Math|Vector|CrossProduct (Math|Vector|Normalize _returnvalue) (Math|Vector|Normalize (- (Transformation|GetActorLocation _array_element) (Transformation|GetActorLocation _vehicle))))))))))
      (for (_array_element_2 _array_index) (Variables|Default|GetSeen%20Opponents)
        (if (< (.OpponentDistance (Utilities|Struct|BreakAI_Opponents_Struct _array_element_2)) (LocalVariables|GetTemp%20Shortest%20Distance))
          (LocalVariables|SetTemp%20Closest%20Opponent%20Index _array_index)
          (LocalVariables|SetTemp%20Shortest%20Distance (.OpponentDistance (Utilities|Struct|BreakAI_Opponents_Struct _array_element_2)))))
      (Variables|Default|SetClosest%20Opponent%20Index (LocalVariables|GetTemp%20Closest%20Opponent%20Index))
      (for (_array_element_3 _array_index_2) (Variables|Default|GetSeen%20Opponents)
        (if (< (Math|Float|Absolute(Float) (.OpponentAngle (Utilities|Struct|BreakAI_Opponents_Struct _array_element_3))) (LocalVariables|GetTemp%20Most%20in%20Front%20Angle))
          (LocalVariables|SetTemp%20Most%20in%20Front%20Opponent%20Index _array_index_2)
          (LocalVariables|SetTemp%20Most%20in%20Front%20Angle (Math|Float|Absolute(Float) (.OpponentAngle (Utilities|Struct|BreakAI_Opponents_Struct _array_element_3))))))
      (Variables|Default|SetMost%20in%20Front%20Opponent%20Index (LocalVariables|GetTemp%20Most%20in%20Front%20Opponent%20Index)))))