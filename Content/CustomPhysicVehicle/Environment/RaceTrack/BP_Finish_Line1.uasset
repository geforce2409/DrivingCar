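; Race track finish line that counts laps and records best lap times for vehicles overlapping its box trigger.
; On a VehicleMesh-tagged overlap, it finds the vehicle's index in BP_GM_Race's Cars array and updates the parallel Laps, LapStartTime and BestLapTime arrays.
; The first crossing starts timing without recording a lap time, and later crossings save faster times and restart the timer.
; It has no direction or checkpoint check, and its player-controlled branch is empty.
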(event OnComponentBeginOverlap(Box)
  (params (OverlappedComponent :type Primitive%20Component%20Object%20Reference) (OtherActor :type Actor%20Object%20Reference) (OtherComp :type Primitive%20Component%20Object%20Reference) (OtherBodyIndex :type Integer) (bFromSweep :type Boolean) (SweepResult :type Hit%20Result%20Structure%20%28by%20ref%29))
  (if (Utilities|Array|ContainsItem (Variables|/Script/Engine.ActorComponent|GetComponentTags OtherComp) "VehicleMesh")
    (bind _asbp_master_vehicle (Utilities|Casting|CastToBP_Master_Vehicle OtherActor))
    (Utilities|Array|SetArrayElem (Variables|/Game/Blueprints/BP_GM_Race.BP_GM_Race_C|GetLaps (stale EventBeginPlay _asbp_gm_race)) (Utilities|Array|FindItem (Variables|/Game/Blueprints/BP_GM_Race.BP_GM_Race_C|GetCars (stale EventBeginPlay _asbp_gm_race)) _asbp_master_vehicle) (+ (Utilities|Array|Get(acopy) (Variables|/Game/Blueprints/BP_GM_Race.BP_GM_Race_C|GetLaps (stale EventBeginPlay _asbp_gm_race)) (Utilities|Array|FindItem (Variables|/Game/Blueprints/BP_GM_Race.BP_GM_Race_C|GetCars (stale EventBeginPlay _asbp_gm_race)) _asbp_master_vehicle)) 1))
    (if (< (- (Utilities|Time|GetGameTimeinSeconds) (Utilities|Array|Get(acopy) (Variables|/Game/Blueprints/BP_GM_Race.BP_GM_Race_C|GetLap%20Start%20Time (stale EventBeginPlay _asbp_gm_race)) (Utilities|Array|FindItem (Variables|/Game/Blueprints/BP_GM_Race.BP_GM_Race_C|GetCars (stale EventBeginPlay _asbp_gm_race)) _asbp_master_vehicle))) (Utilities|Array|Get(acopy) (Variables|/Game/Blueprints/BP_GM_Race.BP_GM_Race_C|GetBest%20Lap%20Time (stale EventBeginPlay _asbp_gm_race)) (Utilities|Array|FindItem (Variables|/Game/Blueprints/BP_GM_Race.BP_GM_Race_C|GetCars (stale EventBeginPlay _asbp_gm_race)) _asbp_master_vehicle)))
      (if (== (Utilities|Array|Get(acopy) (Variables|/Game/Blueprints/BP_GM_Race.BP_GM_Race_C|GetLaps (stale EventBeginPlay _asbp_gm_race)) (Utilities|Array|FindItem (Variables|/Game/Blueprints/BP_GM_Race.BP_GM_Race_C|GetCars (stale EventBeginPlay _asbp_gm_race)) _asbp_master_vehicle)) 1)
        _
        (else
          (Utilities|Array|SetArrayElem (Variables|/Game/Blueprints/BP_GM_Race.BP_GM_Race_C|GetBest%20Lap%20Time (stale EventBeginPlay _asbp_gm_race)) (Utilities|Array|FindItem (Variables|/Game/Blueprints/BP_GM_Race.BP_GM_Race_C|GetCars (stale EventBeginPlay _asbp_gm_race)) _asbp_master_vehicle) (- (Utilities|Time|GetGameTimeinSeconds) (Utilities|Array|Get(acopy) (Variables|/Game/Blueprints/BP_GM_Race.BP_GM_Race_C|GetLap%20Start%20Time (stale EventBeginPlay _asbp_gm_race)) (Utilities|Array|FindItem (Variables|/Game/Blueprints/BP_GM_Race.BP_GM_Race_C|GetCars (stale EventBeginPlay _asbp_gm_race)) _asbp_master_vehicle))) true)))
      (Utilities|Array|SetArrayElem (Variables|/Game/Blueprints/BP_GM_Race.BP_GM_Race_C|GetLap%20Start%20Time (stale EventBeginPlay _asbp_gm_race)) (Utilities|Array|FindItem (Variables|/Game/Blueprints/BP_GM_Race.BP_GM_Race_C|GetCars (stale EventBeginPlay _asbp_gm_race)) _asbp_master_vehicle) (Utilities|Time|GetGameTimeinSeconds) true :!label _label)
      (if (Pawn|IsPlayerControlled (Utilities|Array|Get(acopy) (Variables|/Game/Blueprints/BP_GM_Race.BP_GM_Race_C|GetCars (stale EventBeginPlay _asbp_gm_race)) (Utilities|Array|FindItem (Variables|/Game/Blueprints/BP_GM_Race.BP_GM_Race_C|GetCars (stale EventBeginPlay _asbp_gm_race)) _asbp_master_vehicle)))
        _)
      (elif (== (Utilities|Array|Get(acopy) (Variables|/Game/Blueprints/BP_GM_Race.BP_GM_Race_C|GetLaps (stale EventBeginPlay _asbp_gm_race)) (Utilities|Array|FindItem (Variables|/Game/Blueprints/BP_GM_Race.BP_GM_Race_C|GetCars (stale EventBeginPlay _asbp_gm_race)) _asbp_master_vehicle)) 1)
        (Utilities|Array|SetArrayElem (Variables|/Game/Blueprints/BP_GM_Race.BP_GM_Race_C|GetBest%20Lap%20Time (stale EventBeginPlay _asbp_gm_race)) (Utilities|Array|FindItem (Variables|/Game/Blueprints/BP_GM_Race.BP_GM_Race_C|GetCars (stale EventBeginPlay _asbp_gm_race)) _asbp_master_vehicle) 1.8647120722022892e+18 true)
        (Utilities|Array|SetArrayElem (Variables|/Game/Blueprints/BP_GM_Race.BP_GM_Race_C|GetLap%20Start%20Time (stale EventBeginPlay _asbp_gm_race)) (Utilities|Array|FindItem (Variables|/Game/Blueprints/BP_GM_Race.BP_GM_Race_C|GetCars (stale EventBeginPlay _asbp_gm_race)) _asbp_master_vehicle) (Utilities|Time|GetGameTimeinSeconds) true)
        (else
          (goto _label))))))

(event EventBeginPlay
  (bind _asbp_gm_race (Utilities|Casting|CastToBP_GM_Race (Game|GetGameMode))))

(fn ConstructionScript)